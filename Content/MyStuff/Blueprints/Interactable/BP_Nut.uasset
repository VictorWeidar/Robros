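; BP_Nut is a collectible pickup that adds its BoltValue to the bolt score when the player pawn overlaps it.
; The overlap calls IncrementBoltScore on RoBuddiesGameMode, then destroys the actor.
; Each Tick applies a fixed yaw rotation and calls Play on the Bobbing timeline, whose track is added as a local offset on update.
; The spin is per frame, not scaled by delta time.
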(event Collision|EventActorBeginOverlap
  (params (OtherActor :type Actor%20Object%20Reference))
  (if (== OtherActor (Game|Player|GetPlayerPawn 0))
    (bind _asro_buddies_game_mode (Utilities|Casting|CastToRoBuddiesGameMode (Game|GetGameMode)))
    (Default|IncrementBoltScore _asro_buddies_game_mode (Variables|Default|GetBoltValue))
    (Actor|DestroyActor)))

(event EventTick
  (params (DeltaSeconds :type Float%20%28single-precision%29))
  (Transformation|AddActorLocalRotation "0,3.000000, 0" false false)
  (bind _newtrack_0 (Timeline|Bobbing Play)
    (:Update
      (Transformation|AddActorLocalOffset _newtrack_0 false false))))

(fn ConstructionScript)