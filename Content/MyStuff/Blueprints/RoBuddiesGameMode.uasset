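; RoBuddiesGameMode is the game mode that tracks collected bolts, fuel and active fuel tanks for the game.
; On BeginPlay it creates the W_Score widget for the first player, stores it and adds it to the viewport.
; Events increment the bolt, fuel and active tank counters.
; A separate CheckTotalFuel function, not called within this Blueprint, only prints a message when five tanks are active.
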(event Custom|IncrementFuelScore
  (params (Delta%20Score :type Integer))
  (Variables|Default|SetFuelCurrent (+ Delta%20Score (Variables|Default|GetFuelCurrent))))

(event Custom|IncrementActiveTanks
  (Variables|Default|SetTotalFuelActive (+ (Variables|Default|GetTotalFuelActive) 1)))

(event Custom|IncrementBoltScore
  (params (Delta%20Score :type Integer))
  (Variables|Default|SetBoltsCurrent (+ Delta%20Score (Variables|Default|GetBoltsCurrent))))

(event EventBeginPlay
  (bind _returnvalue (UserInterface|CreateWidget "/Game/MyStuff/Blueprints/UI/W_Score.W_Score_C" (Game|GetPlayerController 0)))
  (bind _output_get (Variables|Default|SetScoreWidget _returnvalue))
  (UserInterface|Viewport|AddtoViewport _output_get 0))

(fn ConstructionScript)

(fn CheckTotalFuel
  (if (== (Variables|Default|GetTotalFuelActive) 5)
    (Development|PrintString "All tanks active")))